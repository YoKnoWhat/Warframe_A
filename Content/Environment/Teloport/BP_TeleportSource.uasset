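; Teleport source actor that moves the player pawn to a referenced target actor when the pawn overlaps it.
; On BeginPlay it writes its Text variable to a TextRender component as a label.
; On overlap it checks that the other actor is player 0's pawn and Target is valid, then teleports it to Target's location with rotation reset to zero.
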(event EventBeginPlay
  (Rendering|Components|TextRender|SetText (Variables|Default|GetTextRender) (Variables|Default|GetText)))

(event Collision|EventActorBeginOverlap
  (params (OtherActor :type Actor%20Object%20Reference))
  (if (and (== OtherActor (Game|Player|GetPlayerPawn 0)) (Utilities|IsValid (Variables|Default|GetTarget)))
    (Transformation|Teleport OtherActor (Transformation|GetActorLocation (Variables|Default|GetTarget)) "0, 0, 0")))

(fn ConstructionScript)