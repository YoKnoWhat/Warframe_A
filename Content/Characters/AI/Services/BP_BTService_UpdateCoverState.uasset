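; Behavior tree service meant to sync an AI's cover state with the cover generator, currently inactive because its Tick event does nothing.
; Disconnected logic would set IsAtCoverPoint from whether the CoverPoint blackboard object is set.
; It would then occupy that point for the owning controller if free, or call ReleaseCover when the key is empty.
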(event EventTick
  (params (OwnerActor :type Actor%20Object%20Reference) (DeltaSeconds :type Float%20%28single-precision%29)))