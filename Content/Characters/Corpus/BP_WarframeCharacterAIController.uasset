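; AI controller for Corpus characters, driving them through the Corpus blackboard and behavior tree.
; On possess it sets the pawn's walk speed, records its spawn position as HomeLocation, resets NoiseLocation, starts the tree and binds perception updates.
; Successful hearing stimuli write NoiseLocation, and sight stimuli set the sensed actor as Target.
; Lost stimuli are ignored, so this controller never clears Target.
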(event Custom|CustomEvent_0
  (params (Actor :type Actor%20Object%20Reference) (Stimulus :type AI%20Stimulus%20Structure))
  (bind (_age _expirationage _strength _stimuluslocation _receiverlocation _tag _bsuccessfullysensed) (Utilities|Struct|BreakAIStimulus Stimulus))
  (if _bsuccessfullysensed
    (bind _returnvalue (Class|AIPerceptionSystem|GetSenseClassforStimulus Stimulus))
    (if (== _returnvalue "/Script/AIModule.AISense_Hearing")
      (AI|Components|Blackboard|SetValueasVector (Variables|Default|GetBlackboard) (Utilities|Name|MakeLiteralName "NoiseLocation") _stimuluslocation)
      (elif (Utilities|ClassIsChildOf _returnvalue "/Script/AIModule.AISense_Sight")
        (Development|PrintString "Enter")
        (AI|Components|Blackboard|SetValueasObject (Variables|Default|GetBlackboard) (Utilities|Name|MakeLiteralName "Target") Actor)))))

(event EventBeginPlay
  (Class|AIController|UseBlackboard "/Game/Characters/Corpus/BB_CorpusBlackboard.BB_CorpusBlackboard"))

(event EventOnPossess
  (params (PossessedPawn :type Pawn%20Object%20Reference))
  (Variables|/Script/Engine.CharacterMovementComponent|SetMaxWalkSpeed (Variables|/Script/Engine.Character|GetCharacterMovement (.AsWarframe%20Character (Utilities|Casting|CastToWarframeCharacter PossessedPawn))) 3e+02)
  (AI|Components|Blackboard|SetValueasVector (Variables|Default|GetBlackboard) (Utilities|Name|MakeLiteralName "HomeLocation") (Transformation|GetActorLocation PossessedPawn))
  (AI|Components|Blackboard|SetValueasVector (Variables|Default|GetBlackboard) (Utilities|Name|MakeLiteralName "NoiseLocation") "0, 0, 0")
  (AI|RunBehaviorTree "/Game/Characters/Corpus/BT_CorpusBehaviorTree.BT_CorpusBehaviorTree")
  (EventDispatchers|AssignOnTargetPerceptionUpdated (Class|AIController|GetAIPerceptionComponent) (delegate Custom|CustomEvent_0))
  (|CallParentFunction PossessedPawn))

(fn ConstructionScript)