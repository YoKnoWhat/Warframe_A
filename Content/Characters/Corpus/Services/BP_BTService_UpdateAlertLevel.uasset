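; Behavior tree service for Corpus AI that sets the AlertLevel blackboard enum to one of three states on each tick.
; A set Target gives the highest level, a non-zero NoiseLocation the middle one, and neither the lowest.
; A cached noise location restarts the alarm timer whenever the noise moves.
; After twenty seconds on the same noise without a target, it clears NoiseLocation and drops to the lowest level.
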(event EventTick
  (params (OwnerActor :type Actor%20Object%20Reference) (DeltaSeconds :type Float%20%28single-precision%29))
  (bind _noiselocation (Variables|Default|GetNoiseLocation))
  (bind _returnvalue (Class|BTFunctionLibrary|GetBlackboardValueasVector _noiselocation))
  (if (!= (Class|BTFunctionLibrary|GetBlackboardValueasObject (Variables|Default|GetTarget)) 0)
    (Variables|Default|SetAlarmTimer 0.0)
    (Class|BTFunctionLibrary|SetBlackboardValueasEnum (Variables|Default|GetAlertLevel) (Utilities|Enum|LiteralenumEAIAlertLevel "NewEnumerator2"))
    (elif (Math|Vector|NotEqual(Vector) _returnvalue "0, 0, 0" 0.0001)
      (if (Math|Vector|NotEqual(Vector) (Variables|Default|GetCachedNoiseLocation) _returnvalue 0.0001)
        (Variables|Default|SetAlarmTimer 0.0)
        (Variables|Default|SetCachedNoiseLocation _returnvalue))
      (Variables|Default|SetAlarmTimer (+ (Variables|Default|GetAlarmTimer) DeltaSeconds))
      (if (> (Variables|Default|GetAlarmTimer) 2e+01)
        (AI|BehaviorTree|SetBlackboardValueasVector (Variables|Default|GetNoiseLocation) "0, 0, 0")
        (Variables|Default|SetAlarmTimer 0.0 :!label _label)
        (Class|BTFunctionLibrary|SetBlackboardValueasEnum (Variables|Default|GetAlertLevel) (Utilities|Enum|LiteralenumEAIAlertLevel "NewEnumerator0"))
        (else
          (Class|BTFunctionLibrary|SetBlackboardValueasEnum (Variables|Default|GetAlertLevel) (Utilities|Enum|LiteralenumEAIAlertLevel "NewEnumerator1"))))
      (else
        (goto _label)))))