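; Behavior tree service for Corpus AI that keeps the NewCoverPoint blackboard key updated with a cover point for the pawn to use.
; On tick it runs the EnvQuery_FindCover EQS query, caching the instance so only one query runs at a time.
; On success, if the top result is unoccupied, it releases the previous point, stores the new one and occupies it with the cached Warframe character.
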(event Custom|OnQueryFinishedEvent
  (params (QueryInstance :type Env%20Query%20Instance%20Blueprint%20Wrapper%20Object%20Reference) (QueryStatus :type EEnvQueryStatus%20Enum :default "Processing"))
  (if (== QueryStatus (Utilities|Enum|LiteralenumEEnvQueryStatus "Success"))
    (if (Class|CoverPoint|IsOccupied (Utilities|Array|Get(acopy) (Class|EnvQueryInstanceWarframeWrapper|GetResultsasCoverPoints (Variables|Default|GetCachedQueryInstance))))
      _
      (else
        (bind _ascover_point (Utilities|Casting|CastToCoverPoint (Class|BTFunctionLibrary|GetBlackboardValueasObject (Variables|Default|GetNewCoverPoint)))
          (:then
            (Class|CoverPoint|Release _ascover_point))
          (:CastFailed
            _))
        (Class|BTFunctionLibrary|SetBlackboardValueasObject (Variables|Default|GetNewCoverPoint) (Utilities|Array|Get(acopy) (Class|EnvQueryInstanceWarframeWrapper|GetResultsasCoverPoints (Variables|Default|GetCachedQueryInstance))))
        (Class|CoverPoint|Occupy (Utilities|Array|Get(acopy) (Class|EnvQueryInstanceWarframeWrapper|GetResultsasCoverPoints (Variables|Default|GetCachedQueryInstance))) (Variables|Default|GetCachedWarframeCharacter)))))
  (Variables|Default|SetCachedQueryInstance 0))

(event EventReceiveTickAI
  (params (OwnerController :type AI%20Controller%20Object%20Reference) (ControlledPawn :type Pawn%20Object%20Reference) (DeltaSeconds :type Float%20%28single-precision%29))
  (if (== 0 (Variables|Default|GetCachedQueryInstance))
    (bind _returnvalue (AI|EQS|RunEQSQuery "/Game/Characters/Corpus/Queries/EnvQuery_FindCover.EnvQuery_FindCover" OwnerController "SingleResult" "/Script/Warframe_A.EnvQueryInstanceWarframeWrapper"))
    (bind _output_get (Variables|Default|SetCachedQueryInstance (.AsEnv%20Query%20Instance%20Warframe%20Wrapper (Utilities|Casting|CastToEnvQueryInstanceWarframeWrapper _returnvalue))))
    (EventDispatchers|BindEventtoOnQueryFinishedEvent _output_get (delegate Custom|OnQueryFinishedEvent))))

(event EventReceiveSearchStartAI
  (params (OwnerController :type AI%20Controller%20Object%20Reference) (ControlledPawn :type Pawn%20Object%20Reference))
  (Variables|Default|SetCachedWarframeCharacter (.AsWarframe%20Character (Utilities|Casting|CastToWarframeCharacter ControlledPawn))))