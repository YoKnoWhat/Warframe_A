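; Behavior tree service for Corpus AI that updates the SafeScore blackboard value.
; On tick, it writes a fixed placeholder-like constant to SafeScore whenever the Target blackboard actor is set.
; An unconnected calculation would derive a clamped score by comparing the controlled pawn's combined health and shield ratio against the target's, but it has no effect.
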(event EventTick
  (params (OwnerActor :type Actor%20Object%20Reference) (DeltaSeconds :type Float%20%28single-precision%29))
  (if (!= (AI|BehaviorTree|GetBlackboardValueasActor (Variables|Default|GetTarget)) 0)
    (Class|BTFunctionLibrary|SetBlackboardValueasFloat (Variables|Default|GetSafeScore) 15.0)))