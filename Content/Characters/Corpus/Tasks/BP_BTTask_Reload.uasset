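; Behavior tree task that makes a Corpus AI character reload its weapon.
; On execute it calls Reload on the Warframe character AI controller.
; Each tick it reads the upper layer of the Corpus state machine and finishes successfully once that layer is no longer in the Reloading state.
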(event EventReceiveExecuteAI
  (params (OwnerController :type AI%20Controller%20Object%20Reference) (ControlledPawn :type Pawn%20Object%20Reference))
  (Class|WarframeCharacterAIController|Reload (.AsWarframe%20Character%20AIController (Utilities|Casting|CastToWarframeCharacterAIController OwnerController))))

(event EventReceiveTickAI
  (params (OwnerController :type AI%20Controller%20Object%20Reference) (ControlledPawn :type Pawn%20Object%20Reference) (DeltaSeconds :type Float%20%28single-precision%29))
  (bind _returnvalue (Class|StateMachineComponent|GetCurrentStateID (.AsCorpus%20State%20Machine%20Component (Utilities|Casting|CastToCorpusStateMachineComponent (Class|WarframeCharacter|GetStateMachine (.AsWarframe%20Character (Utilities|Casting|CastToWarframeCharacter ControlledPawn))))) (Math|Conversions|ToInteger(Byte) (Utilities|Enum|LiteralenumECorpusStateLayer "Upper"))))
  (if (!= _returnvalue (Math|Conversions|ToInteger(Byte) (Utilities|Enum|LiteralenumECorpusUpperState "Reloading")))
    (AI|BehaviorTree|FinishExecute true)))