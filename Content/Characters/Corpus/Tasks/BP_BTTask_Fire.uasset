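; Behavior tree task that makes an AI-controlled character fire its weapon for a timed burst.
; On execute it calls BeginFire on the WarframeCharacterAIController, waits for Duration plus a random extra up to RandomDeviation, then stops firing and finishes successfully.
; On abort it stops firing and finishes the abort, but only if the controlled pawn is still valid.
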(event EventReceiveAbortAI
  (params (OwnerController :type AI%20Controller%20Object%20Reference) (ControlledPawn :type Pawn%20Object%20Reference))
  (Utilities|IsValid ControlledPawn
    (:Is%20Valid
      (Class|WarframeCharacterAIController|StopFire (.AsWarframe%20Character%20AIController (Utilities|Casting|CastToWarframeCharacterAIController OwnerController)))
      (Class|BTTaskBlueprintBase|FinishAbort))))

(event EventReceiveExecuteAI
  (params (OwnerController :type AI%20Controller%20Object%20Reference) (ControlledPawn :type Pawn%20Object%20Reference))
  (bind _aswarframe_character_aicontroller (Utilities|Casting|CastToWarframeCharacterAIController OwnerController))
  (Class|WarframeCharacterAIController|BeginFire _aswarframe_character_aicontroller)
  (Utilities|FlowControl|Delay (+ (Math|Random|RandomFloatinRange 0.0 (Variables|Default|GetRandomDeviation)) (Variables|Default|GetDuration)))
  (Class|WarframeCharacterAIController|StopFire _aswarframe_character_aicontroller)
  (AI|BehaviorTree|FinishExecute true))