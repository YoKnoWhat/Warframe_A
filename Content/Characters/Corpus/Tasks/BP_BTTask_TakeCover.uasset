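; Behavior tree task that puts an AI character into cover at the CoverPoint stored in the blackboard.
; It calls TakeCover on the WarframeCharacterAIController, then snaps the pawn's rotation to the point's wall rotator, offset 90 degrees either way for left or right cover.
; Execute never finishes the task, so it runs until aborted, when it calls LeaveCover and finishes the abort if the pawn is valid.
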(event EventReceiveAbortAI
  (params (OwnerController :type AI%20Controller%20Object%20Reference) (ControlledPawn :type Pawn%20Object%20Reference))
  (Utilities|IsValid ControlledPawn
    (:Is%20Valid
      (Class|WarframeCharacterAIController|LeaveCover (.AsWarframe%20Character%20AIController (Utilities|Casting|CastToWarframeCharacterAIController OwnerController)))
      (Class|BTTaskBlueprintBase|FinishAbort))))

(event EventReceiveExecuteAI
  (params (OwnerController :type AI%20Controller%20Object%20Reference) (ControlledPawn :type Pawn%20Object%20Reference))
  (bind _coverpoint (Variables|Default|GetCoverPoint))
  (bind _returnvalue (Class|BTFunctionLibrary|GetBlackboardValueasObject _coverpoint))
  (bind _ascover_point (Utilities|Casting|CastToCoverPoint _returnvalue))
  (bind _rotatorxtowall (Variables|/Script/Warframe_A.CoverPoint|GetRotatorXToWall _ascover_point))
  (Class|WarframeCharacterAIController|TakeCover (.AsWarframe%20Character%20AIController (Utilities|Casting|CastToWarframeCharacterAIController OwnerController)) _ascover_point)
  (if (or (Variables|/Script/Warframe_A.CoverPoint|GetbLeftCoverCrouched _ascover_point) (Variables|/Script/Warframe_A.CoverPoint|GetbLeftCoverStanding _ascover_point))
    (Transformation|SetActorRotation ControlledPawn (Math|Rotator|CombineRotators _rotatorxtowall "0,-90.000000, 0"))
    (elif (or (Variables|/Script/Warframe_A.CoverPoint|GetbRightCoverCrouched _ascover_point) (Variables|/Script/Warframe_A.CoverPoint|GetbRightCoverStanding _ascover_point))
      (Transformation|SetActorRotation ControlledPawn (Math|Rotator|CombineRotators _rotatorxtowall "0,90.000000, 0"))
      (else
        (Transformation|SetActorRotation ControlledPawn _rotatorxtowall)))))