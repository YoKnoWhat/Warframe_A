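; Behavior tree task that moves an AI-controlled pawn to the cover point stored in the NewCoverPoint blackboard key.
; AIMoveTo runs to the point's location with a small acceptance radius; success records it as OldCoverPoint, while failure fails the task.
; A missing or non-CoverPoint value finishes as success without moving.
; Abort only calls FinishAbort, and debug prints comparing both keys are left disconnected.
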(event EventReceiveExecuteAI
  (params (OwnerController :type AI%20Controller%20Object%20Reference) (ControlledPawn :type Pawn%20Object%20Reference))
  (bind _ascover_point (Utilities|Casting|CastToCoverPoint (Class|BTFunctionLibrary|GetBlackboardValueasObject (Variables|Default|GetNewCoverPoint)))
    (:then
      (AI|AIMoveTo ControlledPawn (Variables|/Script/Warframe_A.CoverPoint|GetLocation _ascover_point) 0 15.0 false
        (:OnSuccess
          (Class|BTFunctionLibrary|SetBlackboardValueasObject (Variables|Default|GetOldCoverPoint) _ascover_point)
          (AI|BehaviorTree|FinishExecute true))
        (:OnFail
          (AI|BehaviorTree|FinishExecute false))))
    (:CastFailed
      (AI|BehaviorTree|FinishExecute true))))

(event EventReceiveAbortAI
  (params (OwnerController :type AI%20Controller%20Object%20Reference) (ControlledPawn :type Pawn%20Object%20Reference))
  (Class|BTTaskBlueprintBase|FinishAbort))