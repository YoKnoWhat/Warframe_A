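; Behavior tree decorator for Corpus AI that passes when the controlled pawn is within a distance band of its target.
; It takes the pawn from the owning Warframe character AI controller and reads the target actor from a blackboard key.
; The check measures horizontal distance only, ignoring height, and requires it to fall strictly between the minimum and maximum distance variables.
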(fn PerformConditionCheck
  (params (OwnerActor :type Actor%20Object%20Reference))
  (bind _aswarframe_character_aicontroller (Utilities|Casting|CastToWarframeCharacterAIController OwnerActor))
  (bind _target (Variables|Default|GetTarget))
  (bind _returnvalue (Pawn|GetControlledPawn _aswarframe_character_aicontroller))
  (bind _returnvalue_2 (AI|BehaviorTree|GetBlackboardValueasActor _target))
  (bind _returnvalue_3 (Transformation|GetActorLocation _returnvalue))
  (bind _returnvalue_4 (Transformation|GetActorLocation _returnvalue_2))
  (bind _returnvalue_5 (- _returnvalue_3 _returnvalue_4))
  (bind _returnvalue_6 (Math|Vector|VectorLengthXY _returnvalue_5))
  (return (and (< (Variables|Default|GetMinDistance) _returnvalue_6) (< _returnvalue_6 (Variables|Default|GetMaxDistance)))))