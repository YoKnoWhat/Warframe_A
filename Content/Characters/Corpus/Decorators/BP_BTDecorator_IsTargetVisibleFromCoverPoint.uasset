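; Behavior tree decorator for Corpus AI, named as a check for whether the target is visible from a cover point, though no visibility test is implemented.
; Its AI condition check only casts the CoverPoint blackboard value to a cover point and returns true when that succeeds.
; A disconnected debug print of the cover point's wall direction and cover-side properties remains in the graph but never runs.
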(fn PerformConditionCheckAI
  (params (OwnerController :type AI%20Controller%20Object%20Reference) (ControlledPawn :type Pawn%20Object%20Reference))
  (bind _ascover_point (Utilities|Casting|CastToCoverPoint (Class|BTFunctionLibrary|GetBlackboardValueasObject (Variables|Default|GetCoverPoint))))
  (return true))