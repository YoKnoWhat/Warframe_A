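; BP_Tenno is a Tenno character Blueprint that starts play armed with an AK47.
; BeginPlay initializes the state machine with starting Common, Upper and Aim enum states, then spawns and initializes BP_AK47, attaches it to the right-hand mesh socket and registers itself as owner, all before calling the parent BeginPlay.
; Tick and construction only call the parent, and the four CastAbility functions are empty stubs.
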(event EventBeginPlay
  (Class|StateMachineComponent|Init (Variables|Default|GetStateMachine) (Utilities|Array|MakeArray (Math|Conversions|ToInteger(Byte) (Utilities|Enum|LiteralenumETennoCommonState "NewEnumerator0")) (Math|Conversions|ToInteger(Byte) (Utilities|Enum|LiteralenumETennoUpperState "NewEnumerator0")) (Math|Conversions|ToInteger(Byte) (Utilities|Enum|LiteralenumETennoAimState "NewEnumerator0"))))
  (bind _returnvalue (Game|SpawnActorfromClass "/Game/Weapons/BP_AK47.BP_AK47_C" (Math|Transform|MakeTransform "0, 0, 0") "Undefined" self 0))
  (Class|WeaponBase|InitBP _returnvalue 13 1)
  (bind _output_get (Variables|Default|SetEquippedWeapon _returnvalue))
  (Transformation|AttachComponentToComponent _output_get (Variables|Character|GetMesh) "socket_hand_r" "KeepRelative" "KeepRelative" "KeepRelative" true)
  (Class|WeaponBase|SetOwningCharacter _output_get self)
  (|CallParentFunction))

(event Collision|EventActorBeginOverlap
  (params (OtherActor :type Actor%20Object%20Reference))
  (|CallParentFunction OtherActor) ; This node is disabled and will not be called.\nDrag off pins to build functionality.
)

(event EventTick
  (params (DeltaSeconds :type Float%20%28single-precision%29))
  (|CallParentFunction DeltaSeconds))

(fn ConstructionScript
  (|CallParentFunction))

(fn CastAbility1
  (params (UseSecondaryMode :type Boolean)))

(fn CastAbility2
  (params (UseSecondaryMode :type Boolean)))

(fn CastAbility3
  (params (UseSecondaryMode :type Boolean)))

(fn CastAbility4
  (params (UseSecondaryMode :type Boolean)))