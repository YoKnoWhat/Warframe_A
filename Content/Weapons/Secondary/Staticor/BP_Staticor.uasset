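; BP_Staticor is a secondary weapon that fires BP_StaticorRound projectiles at a given target.
; Its OnRoundFired function spawns a scaled-down round at the muzzle socket, aimed at the target's impact point, and returns it.
; It also attaches a muzzle flash, draws a brief debug line along the shot, and sets the round's initial projectile speed after spawning.
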(event EventBeginPlay)

(event Collision|EventActorBeginOverlap
  (params (OtherActor :type Actor%20Object%20Reference)))

(event EventTick
  (params (DeltaSeconds :type Float%20%28single-precision%29)))

(fn ConstructionScript)

(fn OnRoundFired
  (params (CurrentTarget :type Hit%20Result%20Structure%20%28by%20ref%29))
  (bind _impactpoint (Collision|BreakHitResult CurrentTarget))
  (bind _staticmesh (Variables|Default|GetStaticMesh))
  (bind _returnvalue (Transformation|GetSocketLocation _staticmesh "socket_muzzle"))
  (bind _returnvalue_2 (Game|SpawnActorfromClass "/Game/Weapons/Rounds/BP_StaticorRound.BP_StaticorRound_C" (Math|Transform|MakeTransform _returnvalue (Math|Conversions|RotationFromXVector (Math|Vector|Normalize (- _impactpoint _returnvalue))) "0.300000,0.300000,0.300000") "Undefined" self 0))
  (Effects|SpawnEmitterAttached "/Game/InfinityBladeEffects/Effects/FX_Monsters/FX_Monster_Chicken/P_ChickenMaster_MuzzleFlash_01.P_ChickenMaster_MuzzleFlash_01" 0 "socket_muzzle" "0, 0, 0" "0, 0, 0" "0.300000,0.300000,0.300000")
  (Rendering|Debug|DrawDebugLine _returnvalue _impactpoint (Utilities|Struct|MakeLinearColor 0.0 1.0 0.0 1.0) 0.5 0.0)
  (Variables|/Script/Engine.ProjectileMovementComponent|SetInitialSpeed (Variables|/Game/Weapons/Rounds/BP_StaticorRound.BP_StaticorRound_C|GetProjectileMovement _returnvalue_2) 5e+03)
  (return _returnvalue_2))