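; BP_StaticorRound is the explosive round for the Staticor weapon, dealing area hits to WarframeCharacters.
; On overlapping any actor other than its Instigator, it sphere-overlaps nearby pawns, calls OnHit on each character except the Instigator, spawns the explosion emitter and destroys itself.
; A line-trace variant of the same explosion, sweeping from LastLocation to the current position, is left unconnected and never runs.
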(event EventBeginPlay)

(event Collision|EventActorBeginOverlap
  (params (OtherActor :type Actor%20Object%20Reference))
  (if (not (== OtherActor (Variables|Default|GetInstigator)))
    (bind _outactors (Collision|SphereOverlapActors (Transformation|GetActorLocation) 8e+02 (Utilities|Array|MakeArray "ObjectTypeQuery3") "/Script/Warframe_A.WarframeCharacter" (Utilities|Array|MakeArray (Variables|Default|GetInstigator))))
    (for _array_element _outactors
      (Class|RoundBase|OnHit (.AsWarframe%20Character (Utilities|Casting|CastToWarframeCharacter _array_element)) (Transformation|GetActorLocation (.AsWarframe%20Character (Utilities|Casting|CastToWarframeCharacter _array_element)))))
    (Effects|SpawnEmitteratLocation "/Game/Weapons/Secondary/Staticor/P_StaticorExplosion.P_StaticorExplosion" (Transformation|GetActorLocation))
    (Actor|DestroyActor)))

(event EventTick
  (params (DeltaSeconds :type Float%20%28single-precision%29)))

(fn ConstructionScript)