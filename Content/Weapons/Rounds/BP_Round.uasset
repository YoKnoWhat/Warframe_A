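; BP_Round is a weapon projectile that detects its own hits by tracing each tick rather than relying on overlap events.
; Each Tick it line traces from LastLocation to its current location against WorldStatic and Pawn objects, ignoring its Instigator; this graph never sets LastLocation.
; A hit WarframeCharacter receives OnHit with the impact point.
; Any hit spawns a shield-fire impact emitter at the round's location and destroys it.
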(event EventBeginPlay)

(event Collision|EventActorBeginOverlap
  (params (OtherActor :type Actor%20Object%20Reference)))

(event EventTick
  (params (DeltaSeconds :type Float%20%28single-precision%29))
  (bind (_outhit _returnvalue) (Collision|LineTraceForObjects (Variables|Default|GetLastLocation) (Transformation|GetActorLocation) (Utilities|Array|MakeArray "ObjectTypeQuery1" "ObjectTypeQuery3") false (Utilities|Array|MakeArray (Variables|Default|GetInstigator)) "None"))
  (if _returnvalue
    (bind _aswarframe_character (Utilities|Casting|CastToWarframeCharacter (.HitActor (Collision|BreakHitResult _outhit)))
      (:then
        (Class|RoundBase|OnHit _aswarframe_character (.ImpactPoint (Collision|BreakHitResult _outhit))))
      (:CastFailed
        _))
    (Effects|SpawnEmitteratLocation "/Game/InfinityBladeEffects/Effects/FX_Mobile/Impacts/P_Impact_Shield_Fire.P_Impact_Shield_Fire" (Transformation|GetActorLocation))
    (Actor|DestroyActor)))

(fn ConstructionScript)