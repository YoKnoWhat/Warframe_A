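; Game mode for the Warframe game that sets up the player's HUD and feeds it damage feedback.
; On BeginPlay it casts player 0 to Warframe and, if valid (a guard for Simulate In Editor), creates the HUD bound to it and initializes its properties.
; OnCharacterDamaged forwards hit location, damage and hit details to the HUD only when the player's Warframe caused the damage.
; The character-spawned event is an empty stub.
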(event Custom|OnCharacterSpawned_1)

(event EventBeginPlay
  (Variables|Default|SetWarframe (.AsWarframe (Utilities|Casting|CastToWarframe (Game|GetPlayerCharacter 0))))
  ;[1 1 1] For SIE
  (if (!= (Variables|Default|GetWarframe) 0)
    (bind _returnvalue (UserInterface|CreateWidget "/Game/UI/UI_HUD.UI_HUD_C" (.AsPlayer%20Controller (Utilities|Casting|CastToPlayerController (Pawn|GetController (Variables|Default|GetWarframe)))) (Variables|Default|GetWarframe)))
    (bind _output_get (Variables|Default|SetMainHUD _returnvalue))
    (UserInterface|Viewport|AddtoViewport _output_get 0)
    (Class|WarframeCharacter|InitPropertiesBP (Variables|Default|GetWarframe) 57)))

(event EventOnCharacterDamaged
  (params (DamageCauser :type Actor%20Object%20Reference) (DamagedCharacter :type Warframe%20Character%20Object%20Reference) (HitLocation :type Vector :default "0, 0, 0") (StatusEffect :type EDamageType%20Enum :default "Begin") (Damage :type Float%20%28single-precision%29) (IsDamageOnShield :type Boolean) (CriticalTier :type Integer))
  (bind _aswarframe_character (Utilities|Casting|CastToWarframeCharacter DamageCauser))
  (if (== _aswarframe_character (Variables|Default|GetWarframe))
    (Default|OnCharacterDamaged (Variables|Default|GetMainHUD) HitLocation StatusEffect Damage IsDamageOnShield CriticalTier)))

(fn ConstructionScript)